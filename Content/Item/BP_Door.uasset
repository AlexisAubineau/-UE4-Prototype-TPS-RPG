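; BP_Door is an interactive door that the player can swing open in either of two directions and close again.
; BoxA and BoxB overlaps with BP_Ganfaul enable or disable the door's input.
; InteractDoor switches StateDoor, choosing the opening side by testing BoxA against the player controller, not the pawn.
; Each side has its own timeline driving Door yaw, played to open and reversed to close.
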(event `self.BoxA.OnComponentBeginOverlap`
  (params (OverlappedComponent :type "PrimitiveComponent Object Reference") (OtherActor :type "Actor Object Reference") (OtherComp :type "PrimitiveComponent Object Reference") (OtherBodyIndex :type Integer) (bFromSweep :type Boolean) (SweepResult :type "HitResult Structure (by ref)"))
  (cast `/Game/Personnage/BP_Ganfaul` OtherActor)
  (`self.EnableInput` (`GameplayStatics.GetPlayerController` 0) :!label _label))

(event `self.BoxB.OnComponentBeginOverlap`
  (params (OverlappedComponent :type "PrimitiveComponent Object Reference") (OtherActor :type "Actor Object Reference") (OtherComp :type "PrimitiveComponent Object Reference") (OtherBodyIndex :type Integer) (bFromSweep :type Boolean) (SweepResult :type "HitResult Structure (by ref)"))
  (cast `/Game/Personnage/BP_Ganfaul` OtherActor)
  (goto _label))

(event `self.BoxA.OnComponentEndOverlap`
  (params (OverlappedComponent :type "PrimitiveComponent Object Reference") (OtherActor :type "Actor Object Reference") (OtherComp :type "PrimitiveComponent Object Reference") (OtherBodyIndex :type Integer))
  (cast `/Game/Personnage/BP_Ganfaul` OtherActor)
  (`self.DisableInput` (`GameplayStatics.GetPlayerController` 0) :!label _label_2))

(event `self.BoxB.OnComponentEndOverlap`
  (params (OverlappedComponent :type "PrimitiveComponent Object Reference") (OtherActor :type "Actor Object Reference") (OtherComp :type "PrimitiveComponent Object Reference") (OtherBodyIndex :type Integer))
  (cast `/Game/Personnage/BP_Ganfaul` OtherActor)
  (goto _label_2))

(event `InputAction|InteractDoor`
  (params (Key :type "Key Structure"))
  (:`Pressed`
    (switch `/Game/Item/E_Door` (`self.stateDoor`)
      (:`NewEnumerator0`
        (if (`PrimitiveComponent.IsOverlappingActor` (`self.BoxA`) (`GameplayStatics.GetPlayerController` 0))
          (set `self.stateDoor` "NewEnumerator1")
          (bind (_direction _newtrack_0) (`Timeline|Timeline_0` :!label _label_3)
            (:`Update`
              (`SceneComponent.K2_SetRelativeRotation` (`self.Door`) (`KismetMathLibrary.MakeRotator` 0.0 0.0 (+ _newtrack_0 1.0)) false false)))
          (else
            (set `self.stateDoor` "NewEnumerator2")
            (bind (_direction_2 _newtrack_0_2) (`Timeline|Timeline_1` :!label _label_4)
              (:`Update`
                (`SceneComponent.K2_SetRelativeRotation` (`self.Door`) (`KismetMathLibrary.MakeRotator` 0.0 0.0 (+ _newtrack_0_2 1.0)) false false))))))
      (:`NewEnumerator1`
        (set `self.stateDoor` "NewEnumerator0")
        (goto _label_3 :!via `Reverse`))
      (:`NewEnumerator2`
        (set `self.stateDoor` "NewEnumerator0")
        (goto _label_4 :!via `Reverse`)))))

(fn `UserConstructionScript`)